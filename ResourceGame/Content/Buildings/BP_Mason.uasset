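; BP_Mason is the mason building, a child Blueprint that overrides its parent's state color and processing hooks.
; SetColorByState sets the Mason component's material: green or red by CanBePlaced while floating, and the normal material when ready, with none assigned for processing.
; StartProcessing and EndProcessing call the parent, then switch the PSFire effect on and off.
; DoProcessing is empty, and the event graph holds only disabled default events.
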(event EventBeginPlay
  (|CallParentFunction) ; This node is disabled and will not be called.\nDrag off pins to build functionality.
)

(event Collision|EventActorBeginOverlap
  (params (OtherActor :type Actor%20Object%20Reference))
  (|CallParentFunction OtherActor) ; This node is disabled and will not be called.\nDrag off pins to build functionality.
)

(event EventTick
  (params (DeltaSeconds :type Float%20%28single-precision%29))
  (|CallParentFunction DeltaSeconds) ; This node is disabled and will not be called.\nDrag off pins to build functionality.
)

(fn ConstructionScript
  (|CallParentFunction))

(fn SetColorbyState
  (bind _result (CallFunction|CanbePlaced))
  (Rendering|Material|SetMaterial (Variables|Default|GetMason) 0 (Utilities|Select :Index (Variables|Default|GetState) :NewEnumerator0 (select _result "/Game/Material/M_Mason_Green.M_Mason_Green" "/Game/Material/M_Mason_Red.M_Mason_Red") :NewEnumerator1 "/Game/Material/M_Mason.M_Mason" :NewEnumerator2 0)))

(fn DoProcessing)

(fn StartProcessing
  (|CallParentFunction)
  (Components|Activation|Activate (Variables|Default|GetPS_Fire) false))

(fn EndProcessing
  (|CallParentFunction)
  (Components|Activation|Deactivate (Variables|Default|GetPS_Fire)))