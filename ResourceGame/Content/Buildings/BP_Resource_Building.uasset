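; BP_Resource_Building is a resource-producing building that starts its child-actor worker's loop when placed.
; StartProcessing sets the PROCESSING state, during which Tick calls DoProcessing, an empty function here.
; EndProcessing returns the building to READY and adds the collected amount of its resource class to BP_GameState.
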(event EventBeginPlay
  (|CallParentFunction) ; This node is disabled and will not be called.\nDrag off pins to build functionality.
)

(event Collision|EventActorBeginOverlap
  (params (OtherActor :type Actor%20Object%20Reference))
  (|CallParentFunction OtherActor) ; This node is disabled and will not be called.\nDrag off pins to build functionality.
)

(event EventTick
  (params (DeltaSeconds :type Float%20%28single-precision%29))
  (|CallParentFunction DeltaSeconds)
  (switch Utilities|FlowControl|Switch|SwitchonE_BuildingState (Variables|Default|GetState)
    (:NewEnumerator2
      (CallFunction|DoProcessing))))

(fn ConstructionScript
  (|CallParentFunction))

(fn PlaceBuilding
  (|CallParentFunction)
  (bind _asbp_worker (Utilities|Casting|CastToBP_Worker (Variables|/Script/Engine.ChildActorComponent|GetChildActor (Variables|Default|GetBP_Worker))))
  (Default|StartLoop _asbp_worker))

(fn DoProcessing)

(fn StartProcessing
  (Variables|Default|SetState "NewEnumerator2"))

(fn EndProcessing
  (params (CollectedAmount :type Integer))
  (Variables|Default|SetState "NewEnumerator1")
  (bind _asbp_game_state (Utilities|Casting|CastToBP_GameState (Game|GetGameState)))
  (Default|AddResourceAmount _asbp_game_state (Variables|Default|GetResource%20Class) CollectedAmount))