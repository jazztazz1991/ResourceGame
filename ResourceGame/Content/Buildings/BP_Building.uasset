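; BP_Building is a placeable building actor that moves through floating, under-construction and ready states.
; It tracks overlapping buildings and allows placement only when none overlap and the game state reports its costs are covered.
; Each tick it colors its bounds by state, green or red while floating to show placement validity.
; Placing it shows a spinning construction indicator until a timer marks it ready.
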(event EventBeginPlay)

(event Collision|EventActorBeginOverlap
  (params (OtherActor :type Actor%20Object%20Reference))
  (bind _asbp_building (Utilities|Casting|CastToBP_Building OtherActor))
  (Utilities|Set|Add (Variables|Default|GetOverlappedBuildings) _asbp_building))

(event EventTick
  (params (DeltaSeconds :type Float%20%28single-precision%29))
  (CallFunction|SetColorbyState)
  (switch Utilities|FlowControl|Switch|SwitchonE_BuildingState (Variables|Default|GetState)
    (:NewEnumerator3
      (Transformation|AddWorldRotation (Variables|Default|GetConstructing) "0.000000,1.000000,0.000000" false false))))

(event Collision|EventActorEndOverlap
  (params (OtherActor :type Actor%20Object%20Reference))
  (bind _asbp_building (Utilities|Casting|CastToBP_Building OtherActor))
  (Utilities|Set|Remove (Variables|Default|GetOverlappedBuildings) _asbp_building))

(fn ConstructionScript)

(fn CanbePlaced
  (bind _asbp_game_state (Utilities|Casting|CastToBP_GameState (Game|GetGameState)))
  (bind _result (Default|AreCostsCovered _asbp_game_state (Variables|Default|GetCosts)))
  (return (and _result (== (Utilities|Set|Length (Variables|Default|GetOverlappedBuildings)) 0))))

(fn SetColorbyState
  (bind _result (CallFunction|CanbePlaced))
  (Rendering|Material|SetMaterial (Variables|Default|GetBounds) 0 (Utilities|Select :Index (Variables|Default|GetState) :NewEnumerator0 (select _result "/Game/Material/M_Green.M_Green" "/Game/Material/M_Red.M_Red") :NewEnumerator1 "/Game/Material/M_White.M_White" :NewEnumerator2 0 :NewEnumerator3 0)))

(fn PlaceBuilding
  (Variables|Default|SetState "NewEnumerator3")
  (Utilities|Time|SetTimerbyFunctionName 0 "EndConstructing" 5.0)
  (Development|SetHiddeninGame (Variables|Default|GetConstructing) false false))

(fn EndConstructing
  (Development|SetHiddeninGame (Variables|Default|GetConstructing) true false)
  (Variables|Default|SetState "NewEnumerator1"))