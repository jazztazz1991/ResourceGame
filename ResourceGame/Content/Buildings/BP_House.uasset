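; BP_House is a placeable house building that pays coin taxes to the player's resources once built.
; It overrides SetColorByState to show green or red materials while floating, based on placement validity, and the normal material when ready.
; EndConstructing runs the parent logic, then starts a non-looping timer that calls PayTaxes after a delay, adding BP_Coin through BP_GameState.
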(event EventBeginPlay
  (|CallParentFunction))

(event Collision|EventActorBeginOverlap
  (params (OtherActor :type Actor%20Object%20Reference))
  (|CallParentFunction OtherActor) ; This node is disabled and will not be called.\nDrag off pins to build functionality.
)

(event EventTick
  (params (DeltaSeconds :type Float%20%28single-precision%29))
  (|CallParentFunction DeltaSeconds) ; This node is disabled and will not be called.\nDrag off pins to build functionality.
)

(fn ConstructionScript
  (|CallParentFunction))

(fn SetColorbyState
  (bind _result (CallFunction|CanbePlaced))
  (Rendering|Material|SetMaterial (Variables|Default|GetHouse) 0 (Utilities|Select :Index (Variables|Default|GetState) :NewEnumerator0 (select _result "/Game/Material/M_House_Green.M_House_Green" "/Game/Material/M_House_Red.M_House_Red") :NewEnumerator1 "/Game/Material/M_House.M_House" :NewEnumerator2 0 :NewEnumerator3 0)))

(fn EndConstructing
  (|CallParentFunction)
  (Utilities|Time|SetTimerbyFunctionName 0 "PayTaxes" 1e+01))

(fn PayTaxes
  (bind _asbp_game_state (Utilities|Casting|CastToBP_GameState (Game|GetGameState)))
  (Default|AddResourceAmount _asbp_game_state "/Game/Resources/BP_Coin.BP_Coin_C" 10))