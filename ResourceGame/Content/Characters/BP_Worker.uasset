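; Worker unit that gathers resources for the BP_Resource_Building that owns it as a child actor.
; A Tick-driven state machine finds the nearest resource within the building's range, walks to it, harvests, hauls the load home and has the building process it.
; Timers end harvesting and processing, while state changes swap animations and tool/cargo visibility.
; Movement uses straight per-tick world offsets, without pathfinding or delta-time scaling.
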(event EventBeginPlay
  (bind _asbp_resource_building (Utilities|Casting|CastToBP_Resource_Building (Actor|GetParentActor)))
  (Variables|Default|SetHome _asbp_resource_building))

(event Collision|EventActorBeginOverlap
  (params (OtherActor :type Actor%20Object%20Reference)))

(event EventTick
  (params (DeltaSeconds :type Float%20%28single-precision%29))
  (switch Utilities|FlowControl|Switch|SwitchonE_Worker_State (Variables|Default|GetState)
    (:NewEnumerator1
      (CallFunction|FindNearbyResource))
    (:NewEnumerator5
      (CallFunction|WalktoResource))
    (:NewEnumerator3
      (CallFunction|GoBackHome))))

(fn ConstructionScript)

(fn WalktoResource
  (bind _returnvalue (Transformation|GetActorLocation))
  (bind _currenttargetresource (Variables|Default|GetCurrentTargetResource))
  (bind _returnvalue_2 (Transformation|GetActorLocation _currenttargetresource))
  (bind _returnvalue_3 (- _returnvalue_2 _returnvalue))
  (Utilities|IsValid (Variables|Default|GetCurrentTargetResource)
    (:Is%20Valid
      ;[1 1 1] Move Towards Target
      (Transformation|AddActorWorldOffset (* (Math|Vector|Normalize _returnvalue_3) (Variables|Default|GetMovementSpeed)))
      ;[1 1 1] Rotate towards target
      (Transformation|SetActorRotation (Math|Rotator|FindLookatRotation _returnvalue_2 _returnvalue))
      (if (<= (Math|Vector|VectorLength _returnvalue_3) (Variables|/Game/Resources/BP_Resource.BP_Resource_C|GetHarvestingDistance (Variables|Default|GetCurrentTargetResource)))
        ;[1 1 1] Change State & Animation
        (CallFunction|StartHarvest)))
    (:Is%20Not%20Valid
      (Variables|Default|SetState "NewEnumerator1"))))

(fn FindNearbyResource
  (bind _returnvalue (Transformation|GetActorLocation))
  (bind _resource_class (Variables|Default|GetResource%20Class))
  (bind _home (Variables|Default|GetHome))
  (bind _range (Variables|/Game/Buildings/BP_Resource_Building.BP_Resource_Building_C|GetRange _home))
  (bind _overlappingactors (Collision|GetOverlappingActors _range _resource_class :!class /Script/Engine.PrimitiveComponent))
  (bind _returnvalue_2 (Actor|FindNearestActor _returnvalue _overlappingactors))
  (Utilities|IsValid _returnvalue_2
    (:Is%20Valid
      (bind _asbp_resource (Utilities|Casting|CastToBP_Resource _returnvalue_2))
      (Variables|Default|SetCurrentTargetResource _asbp_resource)
      (Variables|Default|SetState "NewEnumerator5")
      (Development|SetHiddeninGame (Variables|Default|GetTool) false false)
      (Development|SetHiddeninGame (Variables|Default|GetResource) true false)
      (Components|Animation|PlayAnimation (Variables|SkeletalMeshActor|GetSkeletalMeshComponent) "/Game/Animations/A_Walking.A_Walking" true))
    (:Is%20Not%20Valid
      (Variables|Default|SetState "NewEnumerator3"))))

(fn StartLoop
  (Variables|Default|SetState "NewEnumerator1"))

(fn GoBackHome
  (bind _returnvalue (Transformation|GetActorLocation))
  (bind _home (Variables|Default|GetHome))
  (bind _returnvalue_2 (Transformation|GetActorLocation _home))
  (bind _returnvalue_3 (- _returnvalue_2 _returnvalue))
  (Utilities|IsValid (Variables|Default|GetHome)
    (:Is%20Valid
      ;[1 1 1] Move Towards Target
      (Transformation|AddActorWorldOffset (* (Math|Vector|Normalize _returnvalue_3) (Variables|Default|GetCarrySpeed)))
      ;[1 1 1] Rotate towards target
      (Transformation|SetActorRotation (Math|Rotator|FindLookatRotation _returnvalue_2 _returnvalue))
      ;[1 1 1] Change State & Animation
      (if (<= (Math|Vector|VectorLength _returnvalue_3) 5.0)
        (if (> (Variables|Default|GetUnitsHarvested) 0)
          (CallFunction|StartProcessing)
          (else
            (Variables|Default|SetState "NewEnumerator1")))))))

(fn StartHarvest
  (Utilities|Time|SetTimerbyFunctionName 0 "EndHarvest" 5.0)
  (Variables|Default|SetState "NewEnumerator2")
  (Components|Animation|PlayAnimation (Variables|SkeletalMeshActor|GetSkeletalMeshComponent) "/Game/Animations/A_Mining.A_Mining" true))

(fn EndHarvest
  (bind _currenttargetresource (Variables|Default|GetCurrentTargetResource))
  (Utilities|IsValid (Variables|Default|GetCurrentTargetResource)
    (:Is%20Valid
      (Variables|Default|SetState "NewEnumerator3")
      (Components|Animation|PlayAnimation (Variables|SkeletalMeshActor|GetSkeletalMeshComponent) "/Game/Animations/A_Hauling.A_Hauling" true)
      (Development|SetHiddeninGame (Variables|Default|GetTool) true false)
      (Development|SetHiddeninGame (Variables|Default|GetResource) false false)
      (Utilities|IsValid _currenttargetresource
        (:Is%20Valid
          (bind _collectedamount (Default|Harvest _currenttargetresource (Variables|Default|GetMaxHarvestedUnits)))
          (Variables|Default|SetUnitsHarvested _collectedamount))))
    (:Is%20Not%20Valid
      (Variables|Default|SetState "NewEnumerator1")
      (Components|Animation|PlayAnimation (Variables|SkeletalMeshActor|GetSkeletalMeshComponent) "/Game/Animations/A_Walking.A_Walking" true))))

(fn StartProcessing
  (Variables|Default|SetState "NewEnumerator4")
  (Utilities|Time|SetTimerbyFunctionName 0 "EndProcessing" (Variables|Default|GetProcessingDuration))
  (Default|StartProcessing (Variables|Default|GetHome)))

(fn EndProcessing
  (CallFunction|StartLoop)
  (Default|EndProcessing (Variables|Default|GetHome) (Variables|Default|GetUnitsHarvested))
  (Variables|Default|SetUnitsHarvested 0))